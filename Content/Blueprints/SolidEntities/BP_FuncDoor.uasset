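; BP_FuncDoor is a map-entity door that slides open over two seconds with easing when triggered.
; GetDoorDirectionVector maps the entity's Angle to a sideways or vertical axis, with downward as the fallback.
; OnTriggered moves the mesh to a relative location along that axis, sized from its local bounds minus a small margin, with no closing logic.
; BeginPlay prints the entity's TargetName.
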(event `self.OnTriggered`
  (params (TriggerActor :type "Actor Object Reference") (Caller :type "QEntityActor Object Reference"))
  (bind _entitymeshcomponent (`self.EntityMeshComponent`))
  (bind (_min _max) (`StaticMeshComponent.GetLocalBounds` _entitymeshcomponent))
  (bind _newparam (`self.GetDoorDirectionVector`))
  (`KismetSystemLibrary.MoveComponentTo` _entitymeshcomponent (* (- (- _max _min) (10.0 10.0 10.0)) _newparam) (struct) true true 2.0))

(event `self.ReceiveBeginPlay`
  (`KismetSystemLibrary.PrintString` (`.TargetName` (break `QEntityData` (`QEntityComponent.EntityData` (`self.EntityComponent`))))))

(fn `GetDoorDirectionVector`
  (returns (NewParam :type "Vector Structure"))
  (bind (_entityname _classname _targetname _message _angle) (break `QEntityData` (`QEntityComponent.EntityData` (`self.EntityComponent`))))
  (if (== _angle 0.0)
    (return (0.0 1.0 0.0))
    (elif (== _angle 180.0)
      (return (0.0 -1.0 0.0))
      (elif (== _angle -1.0)
        (return (0.0 0.0 1.0))
        (else
          (return (0.0 0.0 -1.0)))))))

(fn `UserConstructionScript`)